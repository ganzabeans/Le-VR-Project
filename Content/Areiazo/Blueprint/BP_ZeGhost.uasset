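; BP_ZeGhost is a ghost actor that comes to life when its referenced AncientHead is awakened.
; It polls the head's IsAwakened flag every Tick and, while true, enables physics simulation on GhostBody and prints a debug message each frame.
; A ZeGhostMoves timeline that would nudge the root along Y is present but never triggered, so physics alone moves the ghost.
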(event EventBeginPlay)

(event EventTick
  (params (DeltaSeconds :type Float%20%28single-precision%29))
  (CallFunction|CheckifHeadAwakened))

(fn ConstructionScript)

(fn CheckifHeadAwakened
  ;[1 1 1] Detects if head is awakened, then simulates physics once done.
  (if (Variables|/Game/Areiazo/Blueprint/Ancient_Head_BP.Ancient_Head_BP_C|GetisAwakened (Variables|Default|GetAncient%20Head))
    (Physics|SetSimulatePhysics (Variables|Default|GetGhost%20Body) true)
    (Development|PrintString "Ghost is Moving")))