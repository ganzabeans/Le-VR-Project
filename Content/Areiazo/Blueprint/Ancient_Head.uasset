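; Ancient head statue Blueprint that awakens after being hit by thrown rocks and makes its eyes glow.
; Each hit on the Head by a BP_ThrowableRock increments a counter, setting an awakened flag once five hits land, with debug prints.
; Tick checks that flag every frame and activates the two eyeball particle systems while it is set.
; An eye material swap exists but is disconnected.
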(event OnComponentHit(Head)
  (params (HitComponent :type Primitive%20Component%20Object%20Reference) (OtherActor :type Actor%20Object%20Reference) (OtherComp :type Primitive%20Component%20Object%20Reference) (NormalImpulse :type Vector :default "0, 0, 0") (Hit :type Hit%20Result%20Structure%20%28by%20ref%29))
  (Utilities|Casting|CastToBP_ThrowableRock OtherActor)
  (CallFunction|CountUp))

(event EventTick
  (params (DeltaSeconds :type Float%20%28single-precision%29))
  (CallFunction|GlowingEyes))

(fn ConstructionScript)

(fn CountUp
  (bind _rocks_thrown (Variables|Default|GetRocks_Thrown))
  (bind _result (Math|Integer|IncrementInt _rocks_thrown)
    (:%20%20
      (Development|PrintString (Utilities|String|ToString(Integer) _result))
      (if (>= _rocks_thrown 5)
        (Variables|Default|SetisAwakened true)
        (Development|PrintString "Awakened")))))

(fn GlowingEyes
  (if (Variables|Default|GetisAwakened)
    (Components|Activation|Activate (Variables|Default|GetZeEyeBall_Particle) false)
    (Components|Activation|Activate (Variables|Default|GetZeEyeBall_Particle1) false)))