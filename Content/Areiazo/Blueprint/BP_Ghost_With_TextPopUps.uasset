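; Ghost NPC actor that shows floating dialogue, stepping to the next line each time a VR or non-VR player pawn begins overlapping it.
; Construction and Tick copy the current Dialogue array entry to a TextRender, with no bounds check on the advancing index.
; Tick also polls a referenced AncientHead and enables physics on the ghost body once awakened.
; A movement timeline is left unconnected, and AbleToSpeak gates no live logic.
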(event EventTick
  (params (DeltaSeconds :type Float%20%28single-precision%29))
  (CallFunction|CheckifHeadAwakened)
  (bind _dialogue__index_ (CallFunction|ConvertArrayOfTextstoSingleText (Variables|Default|GetDialogue) (Variables|Default|GetDialogue%20Index)))
  (Rendering|Components|TextRender|SetText (Variables|Default|GetTextRender) _dialogue__index_))

(event Collision|EventActorBeginOverlap
  (params (OtherActor :type Actor%20Object%20Reference))
  (Development|PrintString "Hello")
  (Utilities|Casting|CastToBP_Pawn_VR OtherActor
    (:then
      _)
    (:CastFailed
      (Utilities|Casting|CastToBP_Pawn_NonVR_Normal OtherActor)))
  (bind _output_get (Variables|Default|SetAble%20to%20Speak true))
  (Development|PrintString (Utilities|String|ToString(Boolean) _output_get))
  (bind _result (Math|Integer|IncrementInt (Variables|Default|GetDialogue%20Index))
    (:%20%20
      (bind _output_get_2 (Variables|Default|SetDialogue%20Index _result))
      (Development|PrintString (Utilities|String|ToString(Integer) _output_get_2)))))

(event Collision|EventActorEndOverlap
  (params (OtherActor :type Actor%20Object%20Reference))
  (Utilities|Casting|CastToBP_Pawn_VR OtherActor
    (:then
      (Variables|Default|SetAble%20to%20Speak false))
    (:CastFailed
      (Utilities|Casting|CastToBP_Pawn_NonVR_Normal OtherActor))))

(event Input|KeyboardEvents|Q
  (params (Key :type Key%20Structure :default "None")))

(fn ConstructionScript
  (bind _dialogue__index_ (CallFunction|ConvertArrayOfTextstoSingleText (Variables|Default|GetDialogue) (Variables|Default|GetDialogue%20Index)))
  (Rendering|Components|TextRender|SetText (Variables|Default|GetTextRender) _dialogue__index_))

(fn CheckifHeadAwakened
  ;[1 1 1] Detects if head is awakened, then simulates physics once done.
  (if (Variables|/Game/Areiazo/Blueprint/Ancient_Head_BP.Ancient_Head_BP_C|GetisAwakened (Variables|Default|GetAncient%20Head))
    (Physics|SetSimulatePhysics (Variables|Default|GetGhost%20Body) true)
    (Development|PrintString "Ghost is Moving")))

(fn ConvertArrayOfTextstoSingleText
  (params (Dialogue :type Array%20of%20Texts) (Index :type Integer))
  (return (Utilities|Array|Get(acopy) Dialogue Index)))