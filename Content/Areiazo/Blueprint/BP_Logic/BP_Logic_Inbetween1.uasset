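; BP_Logic_Inbetween1 is a one-shot overlap trigger that runs a scripted ghost dialogue and portal reveal when the VR or non-VR player pawn enters it.
; It creates a Diag widget for the Ghost to display the dialogue with facial expressions.
; Timed delays then activate the LocalPortal's next locations, unhide it, move the Ghost to a Waypoint and destroy it.
; Repeat overlaps only print a debug string.
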(event EventBeginPlay)

(event Collision|EventActorBeginOverlap
  (params (OtherActor :type Actor%20Object%20Reference))
  (bind _local_portal (Variables|Default|GetLocal%20Portal))
  (bind _ghost (Variables|Default|GetGhost))
  (Utilities|Casting|CastToBP_Pawn_VR OtherActor
    (:then
      _)
    (:CastFailed
      (Utilities|Casting|CastToBP_Pawn_NonVR_Normal OtherActor)))
  (if (Variables|Default|GetisTriggered)
    (Development|PrintString "Hello")
    (else
      (Variables|Default|SetisTriggered true)
      (bind _returnvalue (UserInterface|CreateWidget "/Game/Areiazo/UI/Diag.Diag_C"))
      (Default|AssignDiag _ghost _returnvalue)
      (UserInterface|Viewport|AddtoViewport _returnvalue 0)
      (Default|DisplayDiag _ghost (Variables|Default|GetDialogue) (Variables|Default|GetFaces))
      (Utilities|FlowControl|Delay 8.0)
      (Default|ActivateNextLocations _local_portal)
      (Rendering|SetActorHiddenInGame _local_portal false)
      (Utilities|FlowControl|Delay 3.0)
      (Default|Moveto _ghost (Transformation|GetWorldLocation (Variables|/Game/Areiazo/Blueprint/Waypoint.Waypoint_C|GetDefaultSceneRoot (Variables|Default|GetWaypoint))))
      (Utilities|FlowControl|Delay 2.0)
      (Actor|DestroyActor _ghost))))

(event EventTick
  (params (DeltaSeconds :type Float%20%28single-precision%29)))

(fn ConstructionScript)