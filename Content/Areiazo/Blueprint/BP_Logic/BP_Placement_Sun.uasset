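; Placement slot for the sun symbol in the inner church passage puzzle, hidden when play begins.
; When a Sun_Symbol_Pickup overlaps it, the pickup is destroyed and the placed symbol becomes visible.
; It then calls Iterator on the referenced BP_Inner_Church_Passage to advance the puzzle and plays a lever-style sound at its location.
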(event EventBeginPlay
  (Rendering|SetActorHiddenInGame (Variables|Default|GetThis%20Actor) true))

(event Collision|EventActorBeginOverlap
  (params (OtherActor :type Actor%20Object%20Reference))
  (Utilities|Casting|CastToSun_Symbol_Pickup OtherActor)
  (Actor|DestroyActor (Variables|Default|GetThat%20Actor))
  (Rendering|SetActorHiddenInGame (Variables|Default|GetThis%20Actor) false)
  (bind _asbp_inner_church_passage (Utilities|Casting|CastToBP_Inner_Church_Passage (Variables|Default|GetInner%20Passage%20Puzzle)))
  (Default|Iterator _asbp_inner_church_passage)
  (Audio|PlaySoundatLocation "/Game/Areiazo/Audio/winchester-lever-action-rifle-lever-movement_MJx16oNO.winchester-lever-action-rifle-lever-movement_MJx16oNO" (Transformation|GetWorldLocation (Variables|Default|GetDefaultSceneRoot)) "0, 0, 0" 1.0 1.0 0.0 0 0 0))

(fn ConstructionScript)