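; Trigger actor, apparently for rock completion, that plays a one-time Ghost dialogue when the player overlaps it.
; Overlap accepts either the VR or normal non-VR pawn.
; The first overlap sets a flag, creates a Diag widget, assigns it to the Ghost, and displays the configured dialogue with matching facial expressions.
; Later overlaps only print a debug string.
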(event EventBeginPlay)

(event Collision|EventActorBeginOverlap
  (params (OtherActor :type Actor%20Object%20Reference))
  (bind _ghost (Variables|Default|GetGhost))
  (Utilities|Casting|CastToBP_Pawn_VR OtherActor
    (:then
      _)
    (:CastFailed
      (Utilities|Casting|CastToBP_Pawn_NonVR_Normal OtherActor)))
  (if (Variables|Default|GetisTriggered)
    (Development|PrintString "Hello")
    (else
      (Variables|Default|SetisTriggered true)
      (bind _returnvalue (UserInterface|CreateWidget "/Game/Areiazo/UI/Diag.Diag_C"))
      (Default|AssignDiag _ghost _returnvalue)
      (UserInterface|Viewport|AddtoViewport _returnvalue 0)
      (Default|DisplayDiag _ghost (Variables|Default|GetDialogue) (Variables|Default|GetFaces)))))

(event EventTick
  (params (DeltaSeconds :type Float%20%28single-precision%29)))

(fn ConstructionScript)