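; Trigger logic actor for the start of the trench section, moving a Ghost character and playing its dialogue.
; BeginPlay places the Ghost at a fixed world position; the first actor overlap hides it and shows a new Diag widget with its conversation and expressions.
; After a delay, LocalTeleport activates its next locations and the Ghost moves to a fixed trench position, then reappears.
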(event EventBeginPlay
  (Transformation|SetWorldLocation (Variables|/Game/Areiazo/Blueprint/BP_GhostDiag.BP_GhostDiag_C|GetDefaultSceneRoot (Variables|Default|Getghost)) "-277856.000000,-75691.000000,-90.000000" false false))

(event Collision|EventActorBeginOverlap
  (params (OtherActor :type Actor%20Object%20Reference))
  (bind _ghost (Variables|Default|Getghost))
  (bind _ghost_2 (Variables|Default|Getghost))
  (if (not (Variables|Default|GetisTriggered))
    (Variables|Default|SetisTriggered true)
    (Default|Hide"!" (Variables|Default|Getghost))
    (bind _returnvalue (UserInterface|CreateWidget "/Game/Areiazo/UI/Diag.Diag_C"))
    (Default|AssignDiag _ghost_2 _returnvalue)
    (UserInterface|Viewport|AddtoViewport _returnvalue 0)
    (Default|DisplayDiag _ghost_2 (Variables|Default|GetGhostDiag) (Variables|Default|GetFaces))
    (Utilities|FlowControl|Delay 1e+01)
    (Default|ActivateNextLocations (Variables|Default|GetLocalTeleport))
    (Default|Moveto _ghost "-275748.000000,-96246.000000,-4908.000000")
    (Utilities|FlowControl|Delay 1.0)
    (Default|Show"!" _ghost)))

(event EventTick
  (params (DeltaSeconds :type Float%20%28single-precision%29)))

(fn ConstructionScript)