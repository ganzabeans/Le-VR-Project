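; BP_Trench2 is a one-shot story trigger actor for a trench section, fired the first time any actor overlaps it.
; It snaps the Ghost companion to a fixed world position, then after a short delay has it display its configured dialogue and expressions.
; After a longer timed wait, it sends the Ghost to a second hardcoded location and activates the next locations on Portal2.
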(event Collision|EventActorBeginOverlap
  (params (OtherActor :type Actor%20Object%20Reference))
  (if (Variables|Default|GetisFirst)
    (Variables|Default|SetisFirst false)
    (Transformation|SetWorldLocation (Variables|/Game/Areiazo/Blueprint/BP_GhostDiag.BP_GhostDiag_C|GetDefaultSceneRoot (Variables|Default|GetGhost)) "-337660.000000,-143812.875000,-12651.573242" false false)
    (Utilities|FlowControl|Delay 2.0)
    (Default|DisplayDiag (Variables|Default|GetGhost) (Variables|Default|GetDialogue) (Variables|Default|GetFaces))
    (Utilities|FlowControl|Delay 12.0)
    (Default|Moveto (Variables|Default|GetGhost) "-403260.000000,-130423.875000,-10275.573242")
    (Default|ActivateNextLocations (Variables|Default|GetPortal2))))

(fn ConstructionScript)