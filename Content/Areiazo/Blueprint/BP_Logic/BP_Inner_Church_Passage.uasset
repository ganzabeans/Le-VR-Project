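; BP_Inner_Church_Passage is a counter-triggered actor, apparently for a church passage, that plays an industrial door or elevator sound.
; The Iterator function increments Counter and prints it, with no caller inside this Blueprint.
; Tick polls Counter and, once it reaches the threshold, plays the sound at the root's location and resets the count.
; The group-movement logic is disconnected, so nothing moves here.
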(event EventBeginPlay)

(event Collision|EventActorBeginOverlap
  (params (OtherActor :type Actor%20Object%20Reference)))

(event EventTick
  (params (DeltaSeconds :type Float%20%28single-precision%29))
  (if (>= (Variables|Default|GetCounter) 3)
    (Variables|Default|SetPlay%20Sound true)
    (if (Variables|Default|GetPlay%20Sound)
      (Audio|PlaySoundatLocation "/Game/Areiazo/Audio/short-industrial-door-elevator-move_zJlznSN_.short-industrial-door-elevator-move_zJlznSN_" (Transformation|GetWorldLocation (Variables|Default|GetDefaultSceneRoot)) "0, 0, 0" 1.0 1.0 0.0 0 0 0)
      (Variables|Default|SetPlay%20Sound false)
      (Variables|Default|SetCounter 0))))

(fn ConstructionScript)

(fn Iterator
  (bind _output_get (Variables|Default|SetCounter (Variables|Default|GetCounter)))
  (bind _result (Math|Integer|IncrementInt _output_get)
    (:%20%20
      (Development|PrintString (Utilities|String|ToString(Integer) _result)))))