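; Rock puzzle logic actor that reacts when a BP_GhostDiag overlaps it by briefly handing the ghost over to physics.
; On overlap it calls SimulatePhysics on its Ghost reference, waits two seconds, then calls TurnOffPhysics.
; It then sends that Ghost to the Waypoint's root location with MoveTo.
; The overlapping actor only gates the sequence, and debug prints report contact or no contact.
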(event EventBeginPlay)

(event Collision|EventActorBeginOverlap
  (params (OtherActor :type Actor%20Object%20Reference))
  (bind _ghost (Variables|Default|GetGhost))
  (Utilities|Casting|CastToBP_GhostDiag OtherActor
    (:then
      (Development|PrintString "Contact")
      (Default|SimulatePhysics _ghost)
      (Utilities|FlowControl|Delay 2.0)
      (Default|TurnOffPhysics _ghost)
      (Default|Moveto _ghost (Transformation|GetWorldLocation (Variables|/Game/Areiazo/Blueprint/Waypoint.Waypoint_C|GetDefaultSceneRoot (Variables|Default|GetWaypoint)))))
    (:CastFailed
      (Development|PrintString "No Contact"))))

(event EventTick
  (params (DeltaSeconds :type Float%20%28single-precision%29)))

(fn ConstructionScript)