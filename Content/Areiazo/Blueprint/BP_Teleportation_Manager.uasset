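; Teleportation manager that tracks named teleport locations and decides whether the player can travel between two of them.
; Two maps keyed by location name store each point's position and active flag, filled through AddLocationVector and toggled by the activate and deactivate functions.
; MovePlayer only returns the destination and a CanMove flag; when both ends are active it deactivates them, so the pair must be reactivated before reuse.
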(event EventBeginPlay)

(event EventTick
  (params (DeltaSeconds :type Float%20%28single-precision%29)))

(fn ConstructionScript)

(fn ActivateNextLocation
  (params (CurrentLocation :type Name) (NextLocation :type Name))
  (Utilities|Map|Add (Variables|Default|GetActiveLocations) CurrentLocation true)
  (Utilities|Map|Add (Variables|Default|GetActiveLocations) NextLocation true))

(fn AddLocationVector
  (params (LocationName :type Name) (Position :type Vector) (makeActive? :type Boolean))
  (Utilities|Map|Add (Variables|Default|GetLocations) LocationName Position)
  (Utilities|Map|Add (Variables|Default|GetActiveLocations) LocationName makeActive?))

(fn DeactivateLocation
  (params (Name :type Name))
  (Utilities|Map|Add (Variables|Default|GetActiveLocations) Name false))

(fn PrintKeysandValues
  (params (Map :type Map%20of%20Names%20to%20Structs))
  (bind _keys (Utilities|Map|Keys Map))
  (for _array_element _keys
    (Development|PrintString (Utilities|String|ToString(Name) _array_element)))
  (bind _values (Utilities|Map|Values Map))
  (for _array_element_2 _values
    (Development|PrintString (Utilities|String|ToString(Vector) _array_element_2))))

(fn IsTeleportActive
  (params (Name :type Name))
  (return (.Value (Utilities|Map|Find (Variables|Default|GetActiveLocations) Name))))

(fn GetLocationVector
  (params (Name :type Name))
  (return (.Value (Utilities|Map|Find (Variables|Default|GetLocations) Name))))

(fn AreTeleportsActive
  (params (teleport1 :type Name) (teleport2 :type Name))
  (bind _activelocations (Variables|Default|GetActiveLocations))
  (return (and (.Value (Utilities|Map|Find _activelocations teleport1)) (.Value (Utilities|Map|Find _activelocations teleport2)))))

(fn DeactivateTeleports
  (params (Teleport1 :type Name) (teleport2 :type Name))
  (bind _activelocations (Variables|Default|GetActiveLocations))
  (Utilities|Map|Add _activelocations Teleport1 false)
  (Utilities|Map|Add _activelocations teleport2 false))

(fn MovePlayer
  (params (Location :type Name) (nextLocation :type Name))
  (bind _active (CallFunction|AreTeleportsActive Location nextLocation))
  (if _active
    (CallFunction|DeactivateTeleports Location nextLocation))
  (return (.Value (Utilities|Map|Find (Variables|Default|GetLocations) nextLocation)) _active))