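; Ancient head puzzle actor that awakens once thrown rocks have struck it more than once.
; Head component hits from Throwable_Rock actors increment a counter, which sets an awakened flag past the threshold and prints debug messages.
; Tick polls that flag, repeatedly applying a new eye material and activating two particle systems, while a guard bool limits the whoosh sound at the head to one play.
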(event OnComponentHit(Head)
  (params (HitComponent :type Primitive%20Component%20Object%20Reference) (OtherActor :type Actor%20Object%20Reference) (OtherComp :type Primitive%20Component%20Object%20Reference) (NormalImpulse :type Vector :default "0, 0, 0") (Hit :type Hit%20Result%20Structure%20%28by%20ref%29))
  (Utilities|Casting|CastToThrowable_Rock OtherActor)
  (CallFunction|HitCounter))

(event EventTick
  (params (DeltaSeconds :type Float%20%28single-precision%29))
  (CallFunction|Awaken))

(fn ConstructionScript)

(fn HitCounter
  (bind _counter (Variables|Default|GetCounter))
  (bind _result (Math|Integer|IncrementInt _counter)
    (:%20%20
      (Development|PrintString (Utilities|String|ToString(Integer) _result))
      (if (> _counter 1)
        (Variables|Default|SetisAwakened true)
        (Development|PrintString "Awakened")))))

(fn Awaken
  (if (Variables|Default|GetisAwakened)
    (Rendering|Material|SetMaterial (Variables|Default|GetEyes) 0 "/Game/AVRFramework/Meshes/UI/Display/M_GlassEdging.M_GlassEdging")
    (Components|Activation|Activate (Variables|Default|GetParticleSystem1) false)
    (Components|Activation|Activate (Variables|Default|GetParticleSystem) false)
    (if (not (Variables|Default|GethasSounded))
      (Audio|PlaySoundatLocation "/Game/Areiazo/Audio/fireball-whoosh_GknWsSNu.fireball-whoosh_GknWsSNu" (Transformation|GetWorldLocation (Variables|Default|GetHead)) "0, 0, 0" 1.0 1.0 0.0 "/Game/Areiazo/Audio/AwakenAttenuation.AwakenAttenuation" 0 0)
      (Variables|Default|SethasSounded true))))