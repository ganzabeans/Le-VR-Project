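; A trigger actor for the trench start that runs a one-time ghost dialogue sequence.
; On the first overlap it hides the Ghost and creates a dialogue widget showing the ghost's speech and faces.
; After a fixed delay it tells LocalTeleport to activate its next locations.
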(event EventBeginPlay)

(event Collision|EventActorBeginOverlap
  (params (OtherActor :type Actor%20Object%20Reference))
  (if (not (Variables|Default|GetisTriggered))
    (Variables|Default|SetisTriggered true)
    (Default|Hide"!" (Variables|Default|Getghost))
    (bind _returnvalue (UserInterface|CreateWidget "/Game/Areiazo/UI/Diag.Diag_C"))
    (Default|DisplayDiag _returnvalue (Variables|Default|GetGhostDiag) (Variables|Default|GetFaces))
    (UserInterface|Viewport|AddtoViewport _returnvalue 0)
    (Utilities|FlowControl|Delay 7.5)
    (Default|ActivateNextLocations (Variables|Default|GetLocalTeleport))))

(event EventTick
  (params (DeltaSeconds :type Float%20%28single-precision%29)))

(fn ConstructionScript)