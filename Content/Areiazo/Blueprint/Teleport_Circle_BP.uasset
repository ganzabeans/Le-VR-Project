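; Teleport circle actor that moves an overlapping actor to a linked named location through a shared TeleportManager.
; On BeginPlay it registers its name, position and starting active state with the manager and plays a chime.
; On overlap, if the manager allows the move, it shows temporary particles at both ends and relocates the actor after a short delay.
; ActivateNextLocations spawns magic effects and tells the manager to activate the next location.
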(event EventBeginPlay
  (Variables|Default|SetCurrentLocation (Variables|Default|GetCurrentLocation))
  (Variables|Default|SetNextLocation (Variables|Default|GetNextLocation))
  (Default|AddLocationVector (Variables|Default|GetTeleportManager) (Variables|Default|GetCurrentLocation) (Transformation|GetWorldLocation (Variables|Default|GetDefaultSceneRoot)) (Variables|Default|GetsetActiveOnStart?))
  (Audio|PlaySoundatLocation "/Game/Areiazo/Audio/magic-chimes-on-wind_f11OGHVO.magic-chimes-on-wind_f11OGHVO" (Transformation|GetWorldLocation (Variables|Default|GetDefaultSceneRoot)) "0, 0, 0" 1.0 1.0 0.0 0 0 0))

(event Collision|EventActorBeginOverlap
  (params (OtherActor :type Actor%20Object%20Reference))
  (bind (_newlocation _canmove) (Default|MovePlayer (Variables|Default|GetTeleportManager) (Variables|Default|GetCurrentLocation) (Variables|Default|GetNextLocation)))
  (if _canmove
    (bind _returnvalue (Effects|SpawnEmitteratLocation "/Game/Areiazo/Art_Assets/ZeBall_Particle.ZeBall_Particle" _newlocation "0, 0, 0" "50.000000,50.000000,50.000000" false))
    (bind _returnvalue_2 (Effects|SpawnEmitteratLocation "/Game/Areiazo/Art_Assets/ZeBall_Particle.ZeBall_Particle" (Transformation|GetWorldLocation (Variables|Default|GetBox)) "0, 0, 0" "50.000000,50.000000,50.000000" false))
    (Utilities|FlowControl|Delay 0.3)
    (Transformation|SetWorldLocation (Variables|/Script/Engine.Actor|GetRootComponent OtherActor) _newlocation false false)
    (Components|DestroyComponent _returnvalue_2)
    (Utilities|FlowControl|Delay 0.3)
    (Components|DestroyComponent _returnvalue)))

(fn ConstructionScript)

(fn ActivateNextLocations
  (bind _particlesystem (Variables|Default|GetParticleSystem))
  (bind _returnvalue (Transformation|GetWorldLocation _particlesystem))
  (Effects|SpawnEmitteratLocation "/Game/Areiazo/Particles/MagicUpsidedown_P_Areiazo.MagicUpsidedown_P_Areiazo" (+ _returnvalue "0, 0,-260.000000") "0, 0, 0" "2.000000,2.000000,2.000000")
  (Effects|SpawnEmitteratLocation "/Game/Areiazo/Particles/MagicUpsidedown_P_Areiazo.MagicUpsidedown_P_Areiazo" (+ _returnvalue "0, 0,100.000000") "0, 0, 0" "2.000000,2.000000,2.000000")
  (Default|ActivateNextLocation (Variables|Default|GetTeleportManager) (Variables|Default|GetCurrentLocation) (Variables|Default|GetNextLocation)))