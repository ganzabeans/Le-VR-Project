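; BLEH_BP is a triggerable test actor, apparently a chair, that bursts into fire and launches a linked chair.
; Its interface trigger prints a debug string, spawns a fire emitter at its mesh and calls LAUNCH on ZaOTHERCHAIR.
; This class's LAUNCH plays a timeline that raises its own ZaOTHERCHAIR reference.
; Each update lerps from the current location toward a point above it, so the rise accumulates.
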(event Custom|LAUNCH
  (bind _zaotherchair (Variables|Default|GetzaOTHERCHAIR))
  (bind _defaultsceneroot (Variables|BLEH_BP_C|GetDefaultSceneRoot _zaotherchair))
  (bind _returnvalue (Transformation|GetWorldLocation _defaultsceneroot))
  (bind __myfirstflowchart (Timeline|Timeline_0 Play)
    (:Update
      (Transformation|SetWorldLocation (Variables|BLEH_BP_C|GetDefaultSceneRoot (Variables|Default|GetzaOTHERCHAIR)) (Math|Vector|Lerp(Vector) _returnvalue (+ _returnvalue "0, 0,50.000000") __myfirstflowchart) false false))))

(event EventBeginPlay)

(event Collision|EventActorBeginOverlap
  (params (OtherActor :type Actor%20Object%20Reference)))

(event EventTick
  (params (DeltaSeconds :type Float%20%28single-precision%29)))

(event EventInterfaceTriggerSingle
  (params (Section :type Struct%20Section%20Structure) (Source :type Actor%20Object%20Reference))
  (Development|PrintString "Pee")
  (Effects|SpawnEmitteratLocation "/Game/ZeFolder/Particles/FireParticle.FireParticle" (Transformation|GetWorldLocation (Variables|Default|GetStaticMesh)))
  (CallFunction|LAUNCH (Variables|Default|GetzaOTHERCHAIR)))

(fn ConstructionScript)