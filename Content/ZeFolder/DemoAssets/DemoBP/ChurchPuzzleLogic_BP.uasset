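; Church puzzle controller that activates on actor overlap and enforces a trigger order across an array of pillars.
; Activation swaps a blast-circle particle for fire, fades up the hint wall's emission by timeline and calls Weee on the linked triggers.
; CheckOrder compares pillar trigger states and calls Restart on a sequence violation, though position zero reaches Restart after its scan.
; Restart restores the circle, fades the hint out and resets triggers and pillars.
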(event Custom|Restart
  (Components|DestroyComponent (Variables|Default|GetFireEmitter))
  (bind _returnvalue (Effects|SpawnEmitteratLocation "/Game/ZeFolder/Particles/BlastCircle_Particle.BlastCircle_Particle" "143.000000,-30.000000,40.000000"))
  (Variables|Default|SetCircleEmittter _returnvalue)
  (bind _1sec (Timeline|Timeline_0 PlayFromStart)
    (:Update
      (Rendering|Material|SetScalarParameterValueonMaterials (Variables|/Game/ZeFolder/DemoAssets/DemoBP/RWall_BP.RWall_BP_C|GetStaticMesh (Variables|Default|GetHintWall)) "Emission" (Math|Float|Lerp 1.0 0.0 _1sec))
      (for _array_element (Variables|Default|GetTriggerArray)
        (Default|NotWeeee _array_element))
      (for _array_element_2 (Variables|Default|GetPillarArray)
        (Default|Reset!!! _array_element_2))
      (Variables|Default|SetisActive false))))

(event EventBeginPlay
  (Variables|Default|SetisActive false)
  (bind _returnvalue (Effects|SpawnEmitteratLocation "/Game/ZeFolder/Particles/BlastCircle_Particle.BlastCircle_Particle" "143.000000,-30.000000,40.000000"))
  (Variables|Default|SetCircleEmittter _returnvalue))

(event EventTick
  (params (DeltaSeconds :type Float%20%28single-precision%29)))

(event Collision|EventActorBeginOverlap
  (params (OtherActor :type Actor%20Object%20Reference))
  (if (not (Variables|Default|GetisActive))
    (bind _returnvalue (Effects|SpawnEmitteratLocation "/Game/ZeFolder/Particles/FireParticle.FireParticle" "150.000000,-30.000000,170.000000" "0, 0, 0" "1.000000,1.000000,1.000000" false))
    (Variables|Default|SetFireEmitter _returnvalue)
    (Components|DestroyComponent (Variables|Default|GetCircleEmittter))
    (bind _1sec (Timeline|oneSecond Play)
      (:Update
        (Rendering|Material|SetScalarParameterValueonMaterials (Variables|/Game/ZeFolder/DemoAssets/DemoBP/RWall_BP.RWall_BP_C|GetStaticMesh (Variables|Default|GetHintWall)) "Emission" (Math|Float|Lerp 0.0 1.0 _1sec))
        (for _array_element (Variables|Default|GetTriggerArray)
          (Default|Weee _array_element))
        (for _array_element_2 (Variables|Default|GetPillarArray)
          _)
        (Variables|Default|SetisActive true)))))

(fn ConstructionScript)

(fn CheckOrder
  (params (Position :type Integer))
  (if (== Position 0)
    (bind _index (Utilities|FlowControl|ForLoopwithBreak 1 9 :!label _label)
      (:LoopBody
        (if (Variables|/Game/ZeFolder/DemoAssets/DemoBP/PillarBP.PillarBP_C|GetisTriggered (Utilities|Array|Get(acopy) (Variables|Default|GetPillarArray) _index))
          (goto _label Break)))
      (:Completed
        (CallFunction|Restart :!label _label_2)))
    (elif (and (Variables|/Game/ZeFolder/DemoAssets/DemoBP/PillarBP.PillarBP_C|GetisTriggered (Utilities|Array|Get(acopy) (Variables|Default|GetPillarArray) Position)) (not (Variables|/Game/ZeFolder/DemoAssets/DemoBP/PillarBP.PillarBP_C|GetisTriggered (Utilities|Array|Get(acopy) (Variables|Default|GetPillarArray) (+ Position -1)))))
      (goto _label_2))))