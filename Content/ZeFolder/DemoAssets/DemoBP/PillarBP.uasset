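; PillarBP is a pillar in an order-based church puzzle that sinks when triggered.
; While the referenced ChurchPuzzle is active, the first interface trigger passes the pillar's Order to CheckOrder and plays a timeline that lowers it, stopping if the puzzle deactivates.
; A Reset event clears the triggered flag and eases it back to its BeginPlay position.
; Both timelines lerp from the current location each update, so movement is incremental.
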(event Custom|Reset!!!
  (Variables|Default|SetisTriggered false)
  (bind _pillardrop (Timeline|Timeline_0 Play)
    (:Update
      (Transformation|SetWorldLocation (Variables|Default|GetDefaultSceneRoot) (Math|Vector|Lerp(Vector) (Transformation|GetWorldLocation (Variables|Default|GetDefaultSceneRoot)) (Variables|Default|GetstartPosition) _pillardrop) false false))))

(event EventInterfaceTriggerSingle
  (params (Section :type Struct%20Section%20Structure) (Source :type Actor%20Object%20Reference))
  (bind _defaultsceneroot (Variables|Default|GetDefaultSceneRoot))
  (bind _returnvalue (Transformation|GetWorldLocation _defaultsceneroot))
  (if (Variables|/Game/ZeFolder/DemoAssets/DemoBP/ChurchPuzzleLogic_BP.ChurchPuzzleLogic_BP_C|GetisActive (Variables|Default|GetchurchPuzzle))
    (if (not (Variables|Default|GetisTriggered))
      (Variables|Default|SetisTriggered true)
      (Default|CheckOrder (Variables|Default|GetchurchPuzzle) (Variables|Default|GetOrder))
      (bind _pillardrop (Timeline|PillarDrop Play)
        (:Update
          (if (Variables|/Game/ZeFolder/DemoAssets/DemoBP/ChurchPuzzleLogic_BP.ChurchPuzzleLogic_BP_C|GetisActive (Variables|Default|GetchurchPuzzle))
            (Transformation|SetWorldLocation (Variables|Default|GetDefaultSceneRoot) (Math|Vector|Lerp(Vector) _returnvalue (+ _returnvalue "0, 0,-4.000000") _pillardrop) false false)
            (else
              (Timeline|PillarDrop Stop))))))))

(event EventBeginPlay
  (Variables|Default|SetstartPosition (Transformation|GetWorldLocation (Variables|Default|GetDefaultSceneRoot))))

(fn ConstructionScript)