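; BP_SymbolTriggerTest is a demo test actor whose Button component gives visual feedback through two custom events, with no caller in this graph.
; The weee event plays a timeline that lerps the material's Emission parameter up.
; The notWeeee event clears Emission, sets Red to full, then fades it out on a second timeline.
; Only notWeeee restarts its timeline; weee uses Play, resuming from the current position.
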(event Custom|notWeeee
  (bind _button (Variables|Default|GetButton))
  (Rendering|Material|SetScalarParameterValueonMaterials _button "Red" 1.0)
  (Rendering|Material|SetScalarParameterValueonMaterials _button "Emission" 0.0)
  (bind _1sec (Timeline|Timeline_1 PlayFromStart)
    (:Update
      (Rendering|Material|SetScalarParameterValueonMaterials (Variables|Default|GetButton) "Red" (Math|Float|Lerp 1.0 0.0 _1sec)))))

(event Custom|weee
  (bind _1sec (Timeline|Timeline_0 Play)
    (:Update
      (Rendering|Material|SetScalarParameterValueonMaterials (Variables|Default|GetButton) "Emission" (Math|Float|Lerp 0.0 1.0 _1sec)))))

(event Collision|EventActorBeginOverlap
  (params (OtherActor :type Actor%20Object%20Reference))
  (|CallParentFunction OtherActor) ; This node is disabled and will not be called.\nDrag off pins to build functionality.
)

(event EventTick
  (params (DeltaSeconds :type Float%20%28single-precision%29))
  (|CallParentFunction DeltaSeconds) ; This node is disabled and will not be called.\nDrag off pins to build functionality.
)

(fn ConstructionScript
  (|CallParentFunction))